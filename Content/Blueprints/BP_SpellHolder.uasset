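; BP_SpellHolder wraps a single spell and gates casting it behind a cooldown and a mana cost.
; Tick accumulates elapsed time up to the spell's cooldown, and Init assigns the spell ready to cast.
; TryLaunchSpell spends mana through the player controller, resets the timer, launches the spell and passes its animation to the player character.
; Failed casts print whether cooldown or mana blocked them.
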(event EventBeginPlay)

(event EventTick
  (params (DeltaSeconds :type Float%20%28single-precision%29))
  (Variables|Default|SetCooldown (Math|Float|Clamp(Float) (+ DeltaSeconds (Variables|Default|GetCooldown)) 0.0 (Variables|/Game/Blueprints/DataAssets/BP_DA_Spell.BP_DA_Spell_C|GetCooldown (Variables|Default|GetSpell)))))

(fn TryLaunchSpell
  (if (>= (Variables|Default|GetCooldown) (Variables|/Game/Blueprints/DataAssets/BP_DA_Spell.BP_DA_Spell_C|GetCooldown (Variables|Default|GetSpell)))
    (bind _canspend (Default|TrySpendMana (CallFunction|GetPlayerController) (Variables|/Game/Blueprints/DataAssets/BP_DA_Spell.BP_DA_Spell_C|GetResourceCost (Variables|Default|GetSpell))))
    (if _canspend
      (Variables|Default|SetCooldown 0.0)
      (Default|LaunchSpell (Variables|Default|GetSpell) (CallFunction|GetPlayerController))
      (Default|LaunchSpell (CallFunction|GetPlayerCharacter) (Variables|/Game/Blueprints/DataAssets/BP_DA_Spell.BP_DA_Spell_C|GetAnimation (Variables|Default|GetSpell)))
      (else
        (Development|PrintString (Utilities|String|Append "Could not cast spell" (Utilities|String|ToString(Name) (Variables|/Game/Blueprints/DataAssets/BP_DA_Spell.BP_DA_Spell_C|GetName (Variables|Default|GetSpell))) " (mana)"))))
    (else
      (Development|PrintString (Utilities|String|Append "Could not cast spell" (Utilities|String|ToString(Name) (Variables|/Game/Blueprints/DataAssets/BP_DA_Spell.BP_DA_Spell_C|GetName (Variables|Default|GetSpell))) " (cooldown)")))))

(fn Init
  (params (Spell :type BP%20DA%20Spell%20Object%20Reference))
  (bind _output_get (Variables|Default|SetSpell Spell))
  (Variables|Default|SetCooldown (Variables|/Game/Blueprints/DataAssets/BP_DA_Spell.BP_DA_Spell_C|GetCooldown _output_get)))
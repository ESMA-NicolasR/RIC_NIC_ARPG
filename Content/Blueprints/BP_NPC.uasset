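; NPC Blueprint for a top-down game that marks itself as available for interaction and switches the camera for dialogue.
; Its Sphere overlap events set and clear NearbyNPC on the player controller when BP_TopDownCharacter enters or leaves.
; The Dialogue event uses a FlipFlop to alternately blend the view target to the NPC and back to the player character.
; It contains no dialogue content, only the camera toggle.
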(event OnComponentBeginOverlap(Sphere)
  (params (OverlappedComponent :type Primitive%20Component%20Object%20Reference) (OtherActor :type Actor%20Object%20Reference) (OtherComp :type Primitive%20Component%20Object%20Reference) (OtherBodyIndex :type Integer) (bFromSweep :type Boolean) (SweepResult :type Hit%20Result%20Structure%20%28by%20ref%29))
  (Utilities|Casting|CastToBP_TopDownCharacter OtherActor)
  (Variables|/Game/TopDown/Blueprints/BP_TopDownController.BP_TopDownController_C|SetNearbyNPC (CallFunction|GetPlayerController) self))

(event OnComponentEndOverlap(Sphere)
  (params (OverlappedComponent :type Primitive%20Component%20Object%20Reference) (OtherActor :type Actor%20Object%20Reference) (OtherComp :type Primitive%20Component%20Object%20Reference) (OtherBodyIndex :type Integer))
  (Utilities|Casting|CastToBP_TopDownCharacter OtherActor)
  (Variables|/Game/TopDown/Blueprints/BP_TopDownController.BP_TopDownController_C|SetNearbyNPC (CallFunction|GetPlayerController) 0))

(event Custom|Dialogue
  (Utilities|FlowControl|FlipFlop
    (:A
      (Game|Player|SetViewTargetwithBlend (CallFunction|GetPlayerController) self 0.5 "VTBlend_Linear" 0.0 false))
    (:B
      (Game|Player|SetViewTargetwithBlend (CallFunction|GetPlayerController) (CallFunction|GetPlayerCharacter) 0.5 "VTBlend_Linear" 0.0 false))))

(event EventBeginPlay)

(event Collision|EventActorBeginOverlap
  (params (OtherActor :type Actor%20Object%20Reference)))

(event EventTick
  (params (DeltaSeconds :type Float%20%28single-precision%29)))

(fn ConstructionScript)